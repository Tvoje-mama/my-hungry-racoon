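; A clickable light actor whose spotlight can be switched on and off with the F key.
; Overlapping the Clickable component enables input from the first player controller, and ending the overlap disables it, without filtering which actor overlaps.
; F toggles the visibility of the spotlight and the root component of Objec together.
; The construction script applies the Color and Visibility variables to set the initial state.
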(event OnComponentBeginOverlap(clickable)
  (params (OverlappedComponent :type Primitive%20Component%20Object%20Reference) (OtherActor :type Actor%20Object%20Reference) (OtherComp :type Primitive%20Component%20Object%20Reference) (OtherBodyIndex :type Integer) (bFromSweep :type Boolean) (SweepResult :type Hit%20Result%20Structure%20%28by%20ref%29))
  (Input|EnableInput (Game|GetPlayerController 0)))

(event OnComponentEndOverlap(clickable)
  (params (OverlappedComponent :type Primitive%20Component%20Object%20Reference) (OtherActor :type Actor%20Object%20Reference) (OtherComp :type Primitive%20Component%20Object%20Reference) (OtherBodyIndex :type Integer))
  (Input|DisableInput (Game|GetPlayerController 0)))

(event Input|KeyboardEvents|F
  (params (Key :type Key%20Structure))
  (:Pressed
    (Rendering|ToggleVisibility (Variables|Default|GetSpotLight) false)
    (Rendering|ToggleVisibility (Variables|/Script/Engine.Actor|GetRootComponent (Variables|Default|Getobjec)) false)))

(fn ConstructionScript
  (bind _spotlight (Variables|Default|GetSpotLight))
  (Rendering|Components|Light|SetLightColor _spotlight (Variables|Default|Getcolor) true)
  (Rendering|SetVisibility _spotlight (Variables|Default|Getvisibility) false))