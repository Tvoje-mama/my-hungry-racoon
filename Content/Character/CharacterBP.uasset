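; Player character Blueprint that handles movement, mouse look, jumping and a hold-to-punch attack.
; Move axes drive movement relative to controller yaw only, while Turn and LookUp feed controller yaw and pitch.
; Holding Punch sets IsPunching and turns on collision for the LeftHand and RightHand components, and releasing it reverts both.
; The construction script snaps those components to the mesh's hand_l and hand_r sockets.
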(event Input|ActionEvents|InputActionJump
  (params (Key :type Key%20Structure))
  ;[1 1 1] Jump control
  (:Pressed
    (Character|Jump)))

(event Input|ActionEvents|InputActionPunch
  (params (Key :type Key%20Structure))
  (bind _righthand (Variables|Default|GetrightHand))
  ;[1 1 1] Biting
  (:Pressed
    (Variables|Default|SetisPunching true)
    (Collision|SetCollisionEnabled _righthand "QueryAndPhysics"))
  (:Released
    (Variables|Default|SetisPunching false)
    (Collision|SetCollisionEnabled _righthand "NoCollision")))

(event Input|AxisEvents|InputAxisMoveForward
  (params (AxisValue :type Float%20%28single-precision%29))
  ;[1 1 1] Movement control
  (Pawn|Input|AddMovementInput (Math|Vector|GetForwardVector (Math|Rotator|MakeRotator 0.0 0.0 (.Yaw (Math|Rotator|BreakRotator (Pawn|GetControlRotation :!class /Script/Engine.Pawn))))) AxisValue false))

(event Input|AxisEvents|InputAxisMoveRight
  (params (AxisValue :type Float%20%28single-precision%29))
  ;[1 1 1] Movement control
  (Pawn|Input|AddMovementInput (Math|Vector|GetRightVector (Math|Rotator|MakeRotator 0.0 0.0 (.Yaw (Math|Rotator|BreakRotator (Pawn|GetControlRotation :!class /Script/Engine.Pawn))))) AxisValue false))

(event Input|AxisEvents|InputAxisTurn
  (params (AxisValue :type Float%20%28single-precision%29))
  ;[1 1 1] Mouse control
  (Pawn|Input|AddControllerYawInput AxisValue))

(event Input|AxisEvents|InputAxisLookUp
  (params (AxisValue :type Float%20%28single-precision%29))
  ;[1 1 1] Mouse control
  (Pawn|Input|AddControllerPitchInput AxisValue))

(fn ConstructionScript
  (bind _mesh (Variables|Character|GetMesh))
  (Transformation|AttachComponentToComponent (Variables|Default|GetleftHand) _mesh "hand_l" "SnapToTarget" "SnapToTarget" "KeepWorld" true)
  (Transformation|AttachComponentToComponent (Variables|Default|GetrightHand) _mesh "hand_r" "SnapToTarget" "SnapToTarget" "KeepWorld" true))